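; Portal door actor that ends a level when the player character presses E while holding the key.
; Overlap stores the character reference and shows a popup, removed after two seconds or on exit, with the delay also re-running the check.
; Tick polls the stored character, which is never cleared on exit.
; FirstLevel opens SecondLevel; any other level shows the win screen with mouse cursor and pauses the game.
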(event `self.ReceiveTick`
  (params (DeltaSeconds :type "Float (single-precision)"))
  ;[1 1 1] Portal Door conditions for each level
  (if (and (`/Game/ThirdPersonBP/Blueprints/ThirdPersonCharacter.isEPressed` (stale `self.ReceiveActorBeginOverlap` _asthird_person_character)) (`/Game/ThirdPersonBP/Blueprints/ThirdPersonCharacter.hasKey` (stale `self.ReceiveActorBeginOverlap` _asthird_person_character))) :!label _label
    (bind _returnvalue (`GameplayStatics.GetCurrentLevelName` true))
    (if (`KismetStringLibrary.EqualEqual_StrStr` _returnvalue "FirstLevel")
      (`GameplayStatics.OpenLevel` "SecondLevel")
      (else
        (bind _returnvalue_2 (`|CreateWidget` "/Game/WidgetBlueprints/WinScreen.WinScreen_C"))
        (`UserWidget.AddToViewport` _returnvalue_2 0)
        (set `PlayerController.bShowMouseCursor` true (`GameplayStatics.GetPlayerController` 0))
        (`GameplayStatics.SetGamePaused` true)))))

(event `self.ReceiveActorBeginOverlap`
  (params (OtherActor :type "Actor Object Reference"))
  ;[1 1 1] Portal Door conditions for each level
  (bind _asthird_person_character (cast `/Game/ThirdPersonBP/Blueprints/ThirdPersonCharacter` OtherActor))
  (bind _returnvalue (`|CreateWidget` "/Game/WidgetBlueprints/PopUpWidget.PopUpWidget_C"))
  (bind _output_get (set `self.PopupWidget` _returnvalue))
  (`UserWidget.AddToViewport` _output_get 0)
  (`KismetSystemLibrary.Delay` 2.0)
  (`Widget.RemoveFromParent` (`self.PopupWidget`))
  (goto _label))

(event `self.ReceiveActorEndOverlap`
  (params (OtherActor :type "Actor Object Reference"))
  ;[1 1 1] Portal Door conditions for each level
  (cast `/Game/ThirdPersonBP/Blueprints/ThirdPersonCharacter` OtherActor)
  (`Widget.RemoveFromParent` (`self.PopupWidget`)))

(fn `UserConstructionScript`)